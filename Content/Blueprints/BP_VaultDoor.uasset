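; BP_VaultDoor is a vault door that animates when anything overlaps its Sphere3 trigger component.
; A first timeline pitches Sphere2 up to a scaled angle, and its Update output feeds a Delay that starts a second timeline moving Sphere1 along Z while rotating it.
; Ending the overlap reverses only the first timeline from its end; the second is never reversed, and the reverse updates also trigger its delayed Play.
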(event `self.Sphere3.OnComponentBeginOverlap`
  (params (OverlappedComponent :type "PrimitiveComponent Object Reference") (OtherActor :type "Actor Object Reference") (OtherComp :type "PrimitiveComponent Object Reference") (OtherBodyIndex :type Integer) (bFromSweep :type Boolean) (SweepResult :type "HitResult Structure (by ref)"))
  (bind (_direction _newtrack_0) (`Timeline|Timeline` :!label _label)
    (:`Update`
      (`SceneComponent.K2_SetRelativeRotation` (`self.Sphere2`) (`KismetMathLibrary.MakeRotator` 0.0 (* _newtrack_0 180.0)) false false)
      (`KismetSystemLibrary.Delay` 1.0)
      (bind (_direction_2 _newtrack_0_2) (`Timeline|Timeline_0`)
        (:`Update`
          (`SceneComponent.K2_SetRelativeLocationAndRotation` (`self.Sphere1`) (`KismetMathLibrary.MakeVector` 0.0 0.0 (* _newtrack_0_2 90.0)) (`KismetMathLibrary.MakeRotator` 0.0 (* _newtrack_0_2 180.0)) false false))))))

(event `self.Sphere3.OnComponentEndOverlap`
  (params (OverlappedComponent :type "PrimitiveComponent Object Reference") (OtherActor :type "Actor Object Reference") (OtherComp :type "PrimitiveComponent Object Reference") (OtherBodyIndex :type Integer))
  (goto _label :!via `ReverseFromEnd`))

(fn `UserConstructionScript`)