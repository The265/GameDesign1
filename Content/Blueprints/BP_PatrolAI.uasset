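; Patrol AI character that roams between actors tagged as patrol points at a randomized walk speed.
; On BeginPlay it gathers and shuffles the tagged actors, then loops AI move requests through them with a short delay, reshuffling after each full pass.
; Failed moves advance to the next point just like successful ones, with debug prints for each result.
; A similar player-chasing MoveTo loop exists but is never triggered in this graph.
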(event `Move To`
  (`|AIMoveTo` self (0.0 0.0 0.0) (`GameplayStatics.GetPlayerCharacter` 0) 200.0
    (:`OnSuccess`
      (`KismetSystemLibrary.PrintString` "Go"))
    (:`OnFail`
      (`KismetSystemLibrary.PrintString` "No")))
  (`KismetSystemLibrary.Delay` 1.0)
  (`self.Move To`))

(event `self.ReceiveBeginPlay`
  (bind _outactors (`GameplayStatics.GetAllActorsOfClassWithTag` "/Script/Engine.Actor" (`self.Patrol Point Tag`)))
  (`KismetSystemLibrary.PrintString` (`KismetStringLibrary.Concat_StrStr` "There Are " (`KismetStringLibrary.Conv_IntToString` (`KismetArrayLibrary.Array_Length` _outactors)) " Patrol Points"))
  (`KismetArrayLibrary.Array_Shuffle` _outactors)
  (set `CharacterMovementComponent.MaxWalkSpeed` (`KismetMathLibrary.Conv_IntToDouble` (* (`KismetMathLibrary.RandomIntegerInRange` 16 24) 25)) (`self.CharacterMovement`))
  (`self.GoToControlPoints`))

(event `GoToControlPoints`
  (`|AIMoveTo` self (`self.K2_GetActorLocation` (`|GetArrayItem` (stale `self.ReceiveBeginPlay` _outactors) (`self.CurrentControlPoint`))) null 200.0
    (:`OnSuccess`
      (`KismetSystemLibrary.PrintString` "Go"))
    (:`OnFail`
      (`KismetSystemLibrary.PrintString` "No")))
  (bind _result (`/Engine/EditorBlueprintResources/StandardMacros.IncrementInt` (`self.CurrentControlPoint`))
    (:`  `
      (if (>= _result (`KismetArrayLibrary.Array_Length` (stale `self.ReceiveBeginPlay` _outactors)))
        (set `self.CurrentControlPoint` 0)
        (`KismetArrayLibrary.Array_Shuffle` (stale `self.ReceiveBeginPlay` _outactors)))
      (`KismetSystemLibrary.Delay` 1.0)
      (`self.GoToControlPoints`))))

(fn `UserConstructionScript`)